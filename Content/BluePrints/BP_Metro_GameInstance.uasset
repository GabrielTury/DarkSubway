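; Game instance for the Metro game that keeps per-level loop counters for three Dark levels.
; SetLoops increments the counter matching the current level name, then finds BP_Dark_Manager and calls its matching SetLevel function.
; The two name switches use differing case labels for the first and third levels, so only Dark 2 matches in both.
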(event `self.ReceiveInit`)

(fn `SetLoops`
  (bind _level1loops (`self.level1Loops`))
  (`KismetSystemLibrary.PrintString` "Ativou SetLoops")
  (bind _returnvalue (`GameplayStatics.GetCurrentLevelName` true))
  (switch `string` _returnvalue
    (:`Dark_1`
      (`KismetSystemLibrary.PrintString` (`KismetStringLibrary.Conv_IntToString` _level1loops))
      (`/Engine/EditorBlueprintResources/StandardMacros.IncrementInt` _level1loops
        (:`  `
          _)))
    (:`Dark_2`
      (`/Engine/EditorBlueprintResources/StandardMacros.IncrementInt` (`self.level2Loops`)
        (:`  `
          _)))
    (:`Dark_3`
      (`/Engine/EditorBlueprintResources/StandardMacros.IncrementInt` (`self.level3Loops`)
        (:`  `
          _))))
  (bind _returnvalue_2 (`GameplayStatics.GetActorOfClass` "/Game/BluePrints/BP_Dark_Manager.BP_Dark_Manager_C"))
  (switch `string` _returnvalue
    (:`Dark`
      (`/Game/BluePrints/BP_Dark_Manager.SetLevel1` _returnvalue_2))
    (:`Dark_2`
      (`/Game/BluePrints/BP_Dark_Manager.SetLevel2` _returnvalue_2))
    (:`L_Dark3`
      (`/Game/BluePrints/BP_Dark_Manager.SetLevel3` _returnvalue_2))))